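; Game mode Blueprint that manages the level's outdoor ambient sound as the world mode changes.
; On BeginPlay it binds ChangeAmbientSound to OnChangeWorldMode and calls it once to start the default L1 ambience.
; Each change stops any current ambience, plays a world-shifting sound at the player's location, then spawns the 2D L1, L2 or L3 loop matching the mode.
; The shift sound is skipped when no ambience is active yet.
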(event `self.ReceiveBeginPlay`
  ;[1 1 1] Ambient Sound Logic
  (add `self.OnChangeWorldMode` (delegate `Change Ambient Sound`))
  (`self.Change Ambient Sound` "None"))

(event `Change Ambient Sound` :!signature `self.OnChangeWorldMode`
  (params (mode :type "WorldModes Enum" :default "None"))
  (bind _currentambient (`self.CurrentAmbient`))
  (bind _ambient_volume (`self.Ambient Volume`))
  ;[1 1 1] Ambient Sound Logic
  (if (`KismetSystemLibrary.IsValid` _currentambient)
    (`AudioComponent.Stop` _currentambient)
    (`GameplayStatics.PlaySoundAtLocation` "/Game/Sound/ALL_magic_spells/ALL_world_shifting.ALL_world_shifting" (`self.K2_GetActorLocation` (`GameplayStatics.GetPlayerPawn` 0)) (struct) 1.0 1.0 0.0 null null null))
  (switch `int` (`KismetMathLibrary.Conv_ByteToInt` mode)
    (:`Default`
      (bind _returnvalue (`GameplayStatics.SpawnSound2D` "/Game/Sound/L1_ambience/L1_outdoor_ambience_01.L1_outdoor_ambience_01" _ambient_volume 1.0 0.0 null :!label _label))
      (bind _output_get (set `self.CurrentAmbient` _returnvalue))
      (`AudioComponent.Play` _output_get 0.0))
    (:`0`
      (goto _label))
    (:`1`
      (bind _returnvalue_2 (`GameplayStatics.SpawnSound2D` "/Game/Sound/L2_ambience/L2_outdoor_ambience_01_new.L2_outdoor_ambience_01_new" _ambient_volume 1.0 0.0 null))
      (bind _output_get_2 (set `self.CurrentAmbient` _returnvalue_2))
      (`AudioComponent.Play` _output_get_2 0.0))
    (:`2`
      (bind _returnvalue_3 (`GameplayStatics.SpawnSound2D` "/Game/Sound/L3_ambience/L3_outdoor_ambience_01.L3_outdoor_ambience_01" _ambient_volume 1.0 0.0 null))
      (bind _output_get_3 (set `self.CurrentAmbient` _returnvalue_3))
      (`AudioComponent.Play` _output_get_3 0.0))))

(event `self.ReceiveTick`
  (params (DeltaSeconds :type "Float (single-precision)")))

(fn `UserConstructionScript`)