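; A box trigger volume that changes the volume of the current ambient sound while an SCharacter is inside it.
; On begin overlap it caches AmbientVolume from BP_SGameModeBase and applies its own Multiplier to the game mode's CurrentAmbient.
; On end overlap it sets the cached value back as the volume multiplier.
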(event `self.Box.OnComponentBeginOverlap`
  (params (OverlappedComponent :type "PrimitiveComponent Object Reference") (OtherActor :type "Actor Object Reference") (OtherComp :type "PrimitiveComponent Object Reference") (OtherBodyIndex :type Integer) (bFromSweep :type Boolean) (SweepResult :type "HitResult Structure (by ref)"))
  (cast `SCharacter` OtherActor)
  (bind _asbp_sgame_mode_base (cast `/Game/MainLevel/BP_SGameModeBase` (`GameplayStatics.GetGameMode`)))
  (set `self.MultiplierCache` (`/Game/MainLevel/BP_SGameModeBase.Ambient Volume` _asbp_sgame_mode_base))
  (`AudioComponent.SetVolumeMultiplier` (`/Game/MainLevel/BP_SGameModeBase.CurrentAmbient` _asbp_sgame_mode_base) (`self.Multiplier`)))

(event `self.Box.OnComponentEndOverlap`
  (params (OverlappedComponent :type "PrimitiveComponent Object Reference") (OtherActor :type "Actor Object Reference") (OtherComp :type "PrimitiveComponent Object Reference") (OtherBodyIndex :type Integer))
  (cast `SCharacter` OtherActor)
  (bind _asbp_sgame_mode_base (cast `/Game/MainLevel/BP_SGameModeBase` (`GameplayStatics.GetGameMode`)))
  (`AudioComponent.SetVolumeMultiplier` (`/Game/MainLevel/BP_SGameModeBase.CurrentAmbient` _asbp_sgame_mode_base) (`self.MultiplierCache`)))

(fn `UserConstructionScript`)