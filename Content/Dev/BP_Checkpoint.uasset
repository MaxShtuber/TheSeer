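; Checkpoint actor that registers itself on the player character when its box is overlapped, lighting up and playing an activation sound.
; Overlap dims the previous checkpoint's mesh without clearing its IsActive; registration and sound run twice when a previous one exists.
; The IsActive flag sets the cube material in the construction script and makes the checkpoint the player's initial one on BeginPlay.
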(event `Deactivate`
  (`PrimitiveComponent.SetMaterial` (`self.Cube`) 0 "/Game/AssetsRo/AprilFinal/mat_inactive_tp.mat_inactive_tp")
  (set `self.IsActive` false))

(event `self.ReceiveBeginPlay`
  (bind _asbp_scharacter_new (cast `/Game/Player/BP_SCharacterNew` (`GameplayStatics.GetPlayerPawn` 0)))
  (if (`self.IsActive`)
    (set `SCharacter.Checkpoint` self _asbp_scharacter_new)))

(event `Activate`
  (`PrimitiveComponent.SetMaterial` (`self.Cube`) 0 "/Game/AssetsRo/Runes/Material_004.Material_004")
  (set `self.IsActive` true))

(event `Play Sound`
  (`GameplayStatics.SpawnSound2D` "/Game/Sound/ALL_game_objects/ALL_checkpoint_activating.ALL_checkpoint_activating" 1.0 1.0 0.0 null))

(event `self.Box.OnComponentBeginOverlap`
  (params (OverlappedComponent :type "PrimitiveComponent Object Reference") (OtherActor :type "Actor Object Reference") (OtherComp :type "PrimitiveComponent Object Reference") (OtherBodyIndex :type Integer) (bFromSweep :type Boolean) (SweepResult :type "HitResult Structure (by ref)"))
  (bind _asscharacter (cast `SCharacter` OtherActor))
  (`|ExecutionSequence`
    (:`then_0`
      (bind _checkpoint (`SCharacter.Checkpoint` _asscharacter))
      (if (`KismetSystemLibrary.IsValid` _checkpoint)
        (`PrimitiveComponent.SetMaterial` (`self.GetComponentByClass` _checkpoint "/Script/Engine.StaticMeshComponent") 0 "/Game/AssetsRo/AprilFinal/mat_inactive_tp.mat_inactive_tp")
        (set `SCharacter.Checkpoint` self _asscharacter :!label _label)
        (`self.Play Sound`)
        (`self.Activate`)))
    (:`then_1`
      (goto _label))))

(fn `UserConstructionScript`
  (if (`self.IsActive`)
    (`self.Activate`)
    (else
      (`self.Deactivate`))))