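; Energy rune pickup that spins in place, flees on the first interaction and is collected on the second.
; The first interaction makes Tick fly it upward and sideways with a trail effect until it passes a height limit, then teleport it to a hard-coded world location where it only rotates.
; The next interaction plays a sound, destroys the actor and notifies BP_SGameModeBase through CallOnRuneTake.
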(event `self.ReceiveBeginPlay`
  (`parent.ReceiveBeginPlay`)
  (`ActorComponent.Activate` (`self.AppearanceEffect`) false)
  (`ActorComponent.Deactivate` (`self.FlyingEffect`)))

(event `self.ReceiveTick`
  (params (DeltaSeconds :type "Float (single-precision)"))
  (`parent.ReceiveTick` DeltaSeconds)
  (if (`self.OnlyRotation`)
    (`self.K2_AddActorLocalRotation` (struct :`Yaw` 1.0))
    (elif (`self.isDisappeared`)
      (`self.K2_SetActorLocation` (-55520.0 -49490.0 3000.0))
      (`ActorComponent.Deactivate` (`self.AppearanceEffect`))
      (`ActorComponent.Deactivate` (`self.FlyingEffect`))
      (set `self.OnlyRotation` true)
      (else
        (`self.K2_AddActorLocalRotation` (struct :`Yaw` 1.0))
        (if (`self.isFlying`)
          (`self.K2_SetActorLocation` (`KismetMathLibrary.MakeVector` (+ (.x (`self.K2_GetActorLocation`)) -50.0) (.y (`self.K2_GetActorLocation`)) (+ (.z (`self.K2_GetActorLocation`)) 30.0)))
          (`ActorComponent.Activate` (`self.FlyingEffect`) false)
          (if (> (.z (`self.K2_GetActorLocation`)) 10000.0)
            (set `self.isDisappeared` true)
            (`ActorComponent.Activate` (`self.AppearanceEffect`) false)))))))

(event `self.OnStartInteract`
  (if (`self.isAlreadyFlown`)
    (`GameplayStatics.PlaySound2D` "/Game/Sound/Magic/ALL_get_new_spell.ALL_get_new_spell" 1.0 1.0 0.0 null null)
    (`self.K2_DestroyActor`)
    (bind _asbp_sgame_mode_base (cast `/Game/MainLevel/BP_SGameModeBase` (`GameplayStatics.GetGameMode`)))
    (`SGameModeBase.OnRuneTake` _asbp_sgame_mode_base "None")
    (else
      (set `self.isFlying` true)
      (set `self.isAlreadyFlown` true))))

(fn `UserConstructionScript`
  (`parent.UserConstructionScript`))