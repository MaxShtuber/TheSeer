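; BP_MusicTrigger is a trigger volume that starts a music track when a player character enters it.
; On Box begin overlap with an SCharacter, it spawns the MusicTrack as a 2D sound at the set Volume, guarded by a flag so it plays only once.
; The end overlap handler only performs the character cast, so leaving the box does not stop the music.
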(event `self.Box.OnComponentBeginOverlap`
  (params (OverlappedComponent :type "PrimitiveComponent Object Reference") (OtherActor :type "Actor Object Reference") (OtherComp :type "PrimitiveComponent Object Reference") (OtherBodyIndex :type Integer) (bFromSweep :type Boolean) (SweepResult :type "HitResult Structure (by ref)"))
  (cast `SCharacter` OtherActor)
  (if (not (`self.IsAlreadyPlayed`))
    (set `self.IsAlreadyPlayed` true)
    (`GameplayStatics.SpawnSound2D` (`self.MusicTrack`) (`self.Volume`) 1.0 0.0 null)))

(event `self.Box.OnComponentEndOverlap`
  (params (OverlappedComponent :type "PrimitiveComponent Object Reference") (OtherActor :type "Actor Object Reference") (OtherComp :type "PrimitiveComponent Object Reference") (OtherBodyIndex :type Integer))
  (cast `SCharacter` OtherActor))

(fn `UserConstructionScript`
  (`parent.UserConstructionScript`))