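; BP_FinalGates is the final gate actor that unlocks while a player holding enough collected runes stands near it.
; When BP_SCharacterNew enters the Sphere trigger with at least nine CollectedRunes, it swaps the Cube to an active power material, plays a 2D portal activation sound and sets IsGatesUnlocked.
; Leaving the sphere reverts the material and clears the flag, so the unlocked state lasts only during overlap.
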(event `self.ReceiveActorBeginOverlap`
  (params (OtherActor :type "Actor Object Reference")))

(event `self.Sphere.OnComponentBeginOverlap`
  (params (OverlappedComponent :type "PrimitiveComponent Object Reference") (OtherActor :type "Actor Object Reference") (OtherComp :type "PrimitiveComponent Object Reference") (OtherBodyIndex :type Integer) (bFromSweep :type Boolean) (SweepResult :type "HitResult Structure (by ref)"))
  (bind _asbp_scharacter_new (cast `/Game/Player/BP_SCharacterNew` OtherActor))
  (if (>= (`KismetArrayLibrary.Array_Length` (`/Game/Player/BP_SCharacterNew.CollectedRunes` _asbp_scharacter_new)) 9)
    (`PrimitiveComponent.SetMaterial` (`self.Cube`) 0 "/Game/AssetsRo/power_teleport/mat_power_active.mat_power_active")
    (`GameplayStatics.SpawnSound2D` "/Game/Sound/Objects/ALL_big_portal_activating.ALL_big_portal_activating" 1.5 1.0 0.0 null)
    (set `self.isGatesUnlocked` true)))

(event `self.Sphere.OnComponentEndOverlap`
  (params (OverlappedComponent :type "PrimitiveComponent Object Reference") (OtherActor :type "Actor Object Reference") (OtherComp :type "PrimitiveComponent Object Reference") (OtherBodyIndex :type Integer))
  (cast `/Game/Player/BP_SCharacterNew` OtherActor)
  (`PrimitiveComponent.SetMaterial` (`self.Cube`) 0 "/Game/AssetsRo/power_teleport/mat_power_inactive.mat_power_inactive")
  (set `self.isGatesUnlocked` false))

(fn `UserConstructionScript`)