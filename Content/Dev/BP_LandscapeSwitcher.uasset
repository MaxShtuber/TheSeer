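; Landscape switcher actor that recolors the level's landscape when the game's world mode changes.
; On BeginPlay it binds to the game mode's world-mode change event and swaps the landscape material for a dynamic instance.
; The handler sets the Snow and Stone vector parameters on the landscape to one of two color sets, chosen by the mode.
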(event `self.ReceiveBeginPlay`
  (bind _asbp_sgame_mode_base (cast `/Game/MainLevel/BP_SGameModeBase` (`GameplayStatics.GetGameMode`)))
  (add `SGameModeBase.OnChangeWorldMode` _asbp_sgame_mode_base (delegate `ChangeLandscapeMaterial`))
  (bind _returnvalue (`KismetMaterialLibrary.CreateDynamicMaterialInstance` (`LandscapeProxy.LandscapeMaterial` (`self.Landscape`))))
  (bind _output_get (set `self.DynMaterial` _returnvalue))
  (set `LandscapeProxy.LandscapeMaterial` _output_get (`self.Landscape`)))

(event `ChangeLandscapeMaterial`
  (params (mode :type "WorldModes Enum" :default "FirstWorld"))
  (switch `int` (`KismetMathLibrary.Conv_ByteToInt` mode)
    (:`0`
      (`LandscapeProxy.SetLandscapeMaterialVectorParameterValue` (`self.Landscape`) "Snow" (`self.Snow Color 1`))
      (`LandscapeProxy.SetLandscapeMaterialVectorParameterValue` (`self.Landscape`) "Stone" (`self.Stone Color 1`)))
    (:`1`
      (`LandscapeProxy.SetLandscapeMaterialVectorParameterValue` (`self.Landscape`) "Snow" (`self.Snow Color 2`))
      (`LandscapeProxy.SetLandscapeMaterialVectorParameterValue` (`self.Landscape`) "Stone" (`self.Stone Color2`)))))

(fn `UserConstructionScript`)