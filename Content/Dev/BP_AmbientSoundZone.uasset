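; BP_AmbientSoundZone is an unfinished actor, named for ambient sound zones, with three box triggers tied to first, second and third world flags.
; Each box's begin-overlap event filters for SCharacter, then checks its matching IsFor…World flag.
; The branches lead nowhere, so no sound logic exists yet, and BeginPlay and the construction script only call their parents.
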(event `self.ReceiveBeginPlay`
  (`parent.ReceiveBeginPlay`))

(event `self.Box1.OnComponentBeginOverlap`
  (params (OverlappedComponent :type "PrimitiveComponent Object Reference") (OtherActor :type "Actor Object Reference") (OtherComp :type "PrimitiveComponent Object Reference") (OtherBodyIndex :type Integer) (bFromSweep :type Boolean) (SweepResult :type "HitResult Structure (by ref)"))
  (cast `SCharacter` OtherActor)
  (if (`self.IsForFirstWorld`)
    _))

(event `self.Box2.OnComponentBeginOverlap`
  (params (OverlappedComponent :type "PrimitiveComponent Object Reference") (OtherActor :type "Actor Object Reference") (OtherComp :type "PrimitiveComponent Object Reference") (OtherBodyIndex :type Integer) (bFromSweep :type Boolean) (SweepResult :type "HitResult Structure (by ref)"))
  (cast `SCharacter` OtherActor)
  (if (`self.IsForSecondWorld`)
    _))

(event `self.Box3.OnComponentBeginOverlap`
  (params (OverlappedComponent :type "PrimitiveComponent Object Reference") (OtherActor :type "Actor Object Reference") (OtherComp :type "PrimitiveComponent Object Reference") (OtherBodyIndex :type Integer) (bFromSweep :type Boolean) (SweepResult :type "HitResult Structure (by ref)"))
  (cast `SCharacter` OtherActor)
  (if (`self.IsForThirdWorld`)
    _))

(fn `UserConstructionScript`
  (`parent.UserConstructionScript`))