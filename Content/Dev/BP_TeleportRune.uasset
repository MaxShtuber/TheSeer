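; BP_TeleportRune is a pickup that unlocks teleport when the player interacts with it.
; OnStartInteract sets IsTeleportUnlocked on BP_SGameModeBase, plays a new-spell sound, destroys the actor, then calls OnRuneTake on the game mode.
; Tick starts a quiet, attenuated pulsating sound at the rune's location every frame rather than using a looping audio component.
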(event `self.OnStartInteract`
  (bind _asbp_sgame_mode_base (cast `/Game/MainLevel/BP_SGameModeBase` (`GameplayStatics.GetGameMode`)))
  (set `/Game/MainLevel/BP_SGameModeBase.IsTeleportUnlocked` true _asbp_sgame_mode_base)
  (`GameplayStatics.PlaySound2D` "/Game/Sound/ALL_magic_spells/ALL_get_new_spell.ALL_get_new_spell" 1.0 1.0 0.0 null null)
  (`self.K2_DestroyActor`)
  (bind _asbp_sgame_mode_base_2 (cast `/Game/MainLevel/BP_SGameModeBase` (`GameplayStatics.GetGameMode`)))
  (`SGameModeBase.OnRuneTake` _asbp_sgame_mode_base_2 "None"))

(event `self.ReceiveTick`
  (params (DeltaSeconds :type "Float (single-precision)"))
  (`GameplayStatics.PlaySoundAtLocation` "/Game/Sound/ALL_game_objects/ALL_pulsating_item_01.ALL_pulsating_item_01" (`self.K2_GetActorLocation`) (`self.K2_GetActorRotation`) 0.1 1.0 0.0 "/Game/Sound/SA_Runes.SA_Runes" null null))

(fn `UserConstructionScript`)