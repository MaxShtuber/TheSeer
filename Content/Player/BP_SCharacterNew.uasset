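; Player character Blueprint for a game with world switching, rune collection and checkpoint teleports.
; Take and drop events spin, shrink and socket-attach carried objects, while the mouse wheel zooms the spring arm.
; Input actions teleport to the active checkpoint, cheat-cycle checkpoints by parsing display names, or cast a gate-locked final spell that opens a rune-count-dependent level.
; Three duplicated timeline-driven helpers show timed reminder text, including for blocked world changes.
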(event `self.ReceiveTick`
  (params (DeltaSeconds :type "Float (single-precision)"))
  ;[1 1 1] Update Taken Object
  (if (`KismetSystemLibrary.IsValid` (`self.CurrentTakenActor`))
    (`self.K2_AddActorLocalRotation` (`self.CurrentTakenActor`) (* (`KismetMathLibrary.MakeRotator` 0.0 0.0 DeltaSeconds) 50.0) false false)))

(event `OnObjectTake_Event_0`
  ;[1 1 1] Take object logic
  (if (`KismetSystemLibrary.IsValid` (`self.CurrentTakenActor`))
    (`ActorComponent.Activate` (`self.Taking Object Effect`) false)
    (`GameplayStatics.SpawnSound2D` "/Game/Sound/Magic/ALL_take_item.ALL_take_item" 1.0 1.0 0.0 null)
    (set `self.Initial Scale` (`self.GetActorScale3D` (`self.CurrentTakenActor`)))
    (bind (_direction _scale _location) (`Timeline|Timeline_0` :!via `PlayFromStart` :!label _label)
      (:`Update`
        (if (`KismetSystemLibrary.IsValid` (`self.CurrentTakenActor`))
          (`self.SetActorScale3D` (`self.CurrentTakenActor`) (`KismetMathLibrary.VLerp` (/ (`self.Initial Scale`) (10.0 10.0 10.0)) (`self.GetActorScale3D` (`self.CurrentTakenActor`)) _scale))
          (`self.K2_SetActorLocation` (`self.CurrentTakenActor`) (`KismetMathLibrary.VLerp` (`SceneComponent.GetSocketLocation` (`self.Mesh`) (`self.AttachObjectSocketName`)) (`self.K2_GetActorLocation` (`self.CurrentTakenActor`)) _location) false false)
          (else
            (goto _label :!via `Stop`))))
      (:`Finished`
        (`self.K2_SetActorLocation` (`self.CurrentTakenActor`) (`SceneComponent.GetSocketLocation` (`self.Mesh`) (`self.AttachObjectSocketName`)) false false)
        (`self.K2_AttachToComponent` (`self.CurrentTakenActor`) (`self.Mesh`) (`self.AttachObjectSocketName`) "SnapToTarget" "KeepWorld" "KeepWorld" true)))))

(event `OnObjectDrop_Event_0`
  ;[1 1 1] Take object logic
  (`self.SetActorScale3D` (`self.CurrentTakenActor`) (`self.Initial Scale`))
  (set `self.CurrentTakenActor` null)
  (`GameplayStatics.SpawnSound2D` "/Game/Sound/Magic/ALL_drop_item.ALL_drop_item" 1.0 1.0 0.0 null))

(event `self.ReceiveBeginPlay`
  ;[1 1 1] Changing World Restriction Reminder
  (`ActorComponent.Deactivate` (`self.FinalSpellEffect`))
  (add `self.UnableToChangeWorld` (delegate `UnableToChangeWorld_Event_0`))
  ;[1 1 1] Take object logic
  (add `self.OnObjectTake` (delegate `OnObjectTake_Event_0`))
  (add `self.OnObjectDrop` (delegate `OnObjectDrop_Event_0`)))

(event `UnableToChangeWorld_Event_0`
  (bind _reminder (`self.Reminder`))
  (bind _reminder_2 (`self.Reminder`))
  ;[1 1 1] Changing World Restriction Reminder
  (`GameplayStatics.SpawnSound2D` "/Game/Sound/Magic/ALL_magic_wind_reminder.ALL_magic_wind_reminder" 0.05 1.0 0.0 null)
  (`KismetSystemLibrary.PrintString` "Unable to change World")
  (if (not (`KismetSystemLibrary.IsValid` _reminder))
    (bind _returnvalue (`|CreateWidget` "/Game/MainLevel/WBP_TextReminder.WBP_TextReminder_C"))
    (set `self.Reminder` _returnvalue)
    (`UserWidget.AddToViewport` (`self.Reminder`) 0))
  (`TextBlock.SetText` (`/Game/MainLevel/WBP_TextReminder.TextForRemider` _reminder) "Здесь что-то мешает переместиться в другой мир!")
  (`Widget.SetIsEnabled` _reminder true)
  (`Widget.SetVisibility` _reminder "Visible")
  (`Timeline|Timeline_1` :!via `PlayFromStart`
    (:`Finished`
      (`Widget.SetIsEnabled` _reminder_2 false)
      (`Widget.SetVisibility` _reminder_2 "Hidden"))))

(event `InputAxisKey|MouseWheelAxis`
  (params (AxisValue :type "Float (single-precision)"))
  (bind _springarmcomponent (`self.SpringArmComponent`))
  ;[1 1 1] Third - First Person Camera via Mouse Scroll
  (if (<= (`SpringArmComponent.TargetArmLength` (`self.SpringArmComponent`)) 100.0)
    (set `self.AxisMultiplier` 180.0)
    (else
      (set `self.AxisMultiplier` 10.0)))
  (set `SpringArmComponent.TargetArmLength` (`KismetMathLibrary.FClamp` (+ (* AxisValue (`self.AxisMultiplier`)) (`SpringArmComponent.TargetArmLength` _springarmcomponent)) -80.0 500.0) _springarmcomponent))

(event `InputAction|Teleport`
  (params (Key :type "Key Structure"))
  (bind _checkpoint (`self.Checkpoint`))
  ;[1 1 1] Teleport
  (:`Pressed`
    (bind _asbp_sgame_mode_base (cast `/Game/MainLevel/BP_SGameModeBase` (`GameplayStatics.GetGameMode`)))
    (if (`/Game/MainLevel/BP_SGameModeBase.IsTeleportUnlocked` _asbp_sgame_mode_base)
      (if (`KismetSystemLibrary.IsValid` _checkpoint)
        (`GameplayStatics.SpawnSound2D` "/Game/Sound/Magic/ALL_teleport.ALL_teleport" 1.0 1.0 0.0 null)
        (`ActorComponent.Activate` (`self.ChangeWorldEffect`) false)
        (`self.K2_TeleportTo` (+ (`self.K2_GetActorLocation` _checkpoint) (0.0 0.0 100.0)))))))

(event `InputAction|Cheat`
  (params (Key :type "Key Structure"))
  (bind _reminder (`self.Reminder`))
  (bind _reminder_2 (`self.Reminder`))
  (bind _returnvalue (`KismetSystemLibrary.GetDisplayName` (`self.Checkpoint`)))
  (bind _returnvalue_2 (`KismetStringLibrary.Conv_StringToInt` (`KismetStringLibrary.GetSubstring` _returnvalue 13 2)))
  ;[1 1 1] Cheat codes
  (:`Pressed`
    (bind _asbp_checkpoint (castclass `/Game/Dev/BP_Checkpoint` "/Game/Dev/BP_Checkpoint.BP_Checkpoint_C"))
    (bind _outactors (`GameplayStatics.GetAllActorsOfClass` _asbp_checkpoint))
    (for _array_element _outactors
      (`/Game/Dev/BP_Checkpoint.Deactivate` _array_element))
    (if (== _returnvalue_2 (`KismetArrayLibrary.Array_Length` _outactors))
      (set `self.CheckPointNumber` 0)
      (else
        (set `self.CheckPointNumber` _returnvalue_2)))
    (for _array_element_2 _outactors
      (if (== (`KismetSystemLibrary.GetDisplayName` _array_element_2) (`KismetStringLibrary.Concat_StrStr` (`KismetStringLibrary.GetSubstring` _returnvalue 0 13) (`KismetStringLibrary.Conv_IntToString` (+ (`self.CheckPointNumber`) 1))))
        (bind _output_get (set `self.Checkpoint` _array_element_2))
        (`/Game/Dev/BP_Checkpoint.Activate` _array_element_2)
        (`/Game/Dev/BP_Checkpoint.Play Sound` _array_element_2)
        (if (not (`KismetSystemLibrary.IsValid` _reminder))
          (bind _returnvalue_3 (`|CreateWidget` "/Game/MainLevel/WBP_TextReminder.WBP_TextReminder_C"))
          (set `self.Reminder` _returnvalue_3)
          (`UserWidget.AddToViewport` (`self.Reminder`) 0))
        (bind _returnvalue_4 (`KismetSystemLibrary.GetDisplayName` _output_get))
        (`TextBlock.SetText` (`/Game/MainLevel/WBP_TextReminder.TextForRemider` _reminder) (`KismetTextLibrary.Conv_StringToText` (`KismetStringLibrary.Concat_StrStr` "Активирован следующий телепорт. " _returnvalue_4)))
        (`Widget.SetIsEnabled` _reminder true)
        (`Widget.SetVisibility` _reminder "Visible")
        (`Timeline|Timeline_3` :!via `PlayFromStart`
          (:`Finished`
            (`Widget.SetIsEnabled` _reminder_2 false)
            (`Widget.SetVisibility` _reminder_2 "Hidden")))))
    (`KismetSystemLibrary.PrintString` "Next Teleport is activated")
    (`KismetSystemLibrary.PrintString` _returnvalue_4)))

(event `InputAction|Final Spell`
  (params (Key :type "Key Structure"))
  (bind _reminder (`self.Reminder`))
  (bind _reminder_2 (`self.Reminder`))
  (bind _returnvalue (`KismetStringLibrary.Conv_IntToString` (`KismetArrayLibrary.Array_Length` (`self.CollectedRunes`))))
  (bind _returnvalue_2 (`KismetStringLibrary.Concat_StrStr` "Сначала нужно найти все руны" ": " _returnvalue " из " "10 найдено"))
  ;[1 1 1] Final Level Downloading
  (:`Pressed`
    (bind _returnvalue_3 (`GameplayStatics.GetActorOfClass` "/Game/Dev/BP_FinalGates.BP_FinalGates_C"))
    (if (`/Game/Dev/BP_FinalGates.isGatesUnlocked` _returnvalue_3)
      (set `self.Options` _returnvalue)
      (`GameplayStatics.SpawnSound2D` "/Game/Sound/Magic/ALL_final_magical_spell.ALL_final_magical_spell" 0.2 1.0 0.0 null)
      (`ActorComponent.Activate` (`self.FinalSpellEffect`) false)
      (`SkeletalMeshComponent.PlayAnimation` (`self.Mesh`) "/Game/AssetsRo/Character/Animations/Standing_Cast_Spell_mixamo_com.Standing_Cast_Spell_mixamo_com" true)
      (`KismetSystemLibrary.Delay` 7.0)
      (`KismetSystemLibrary.PrintString` "LOADING")
      (if (> (`KismetArrayLibrary.Array_Length` (`self.CollectedRunes`)) 9)
        (`GameplayStatics.OpenLevel` "FinalLevel2" false (`self.Options`))
        (else
          (`GameplayStatics.OpenLevel` "FinalLevel1" false (`self.Options`))))
      (else
        (`KismetSystemLibrary.PrintString` _returnvalue_2)
        (if (not (`KismetSystemLibrary.IsValid` _reminder))
          (bind _returnvalue_4 (`|CreateWidget` "/Game/MainLevel/WBP_TextReminder.WBP_TextReminder_C"))
          (set `self.Reminder` _returnvalue_4)
          (`UserWidget.AddToViewport` (`self.Reminder`) 0))
        (`TextBlock.SetText` (`/Game/MainLevel/WBP_TextReminder.TextForRemider` _reminder) (`KismetTextLibrary.Conv_StringToText` _returnvalue_2))
        (`Widget.SetIsEnabled` _reminder true)
        (`Widget.SetVisibility` _reminder "Visible")
        (`Timeline|Timeline_2` :!via `PlayFromStart`
          (:`Finished`
            (`Widget.SetIsEnabled` _reminder_2 false)
            (`Widget.SetVisibility` _reminder_2 "Hidden")))))))

(fn `UserConstructionScript`)